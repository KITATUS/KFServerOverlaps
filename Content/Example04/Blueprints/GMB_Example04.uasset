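; Game mode for Example04 that spawns and possesses a KF_Example04_Char for each starting player who has no pawn.
; The spawn transform comes from the first existing character of that class, falling back to the first PlayerStart.
; A random horizontal offset places newcomers near that point, with collision handling that adjusts position if possible but always spawns.
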(event EventHandleStartingNewPlayer
  (params (NewPlayer :type Player%20Controller%20Object%20Reference))
  (Variables|Default|SetLocal_NewPlayer NewPlayer)
  (Utilities|IsValid (Pawn|GetControlledPawn (Variables|Default|GetLocal_NewPlayer))
    (:Is%20Not%20Valid
      (Variables|Default|SetSpawnTransform "")
      (bind _outactors (Actor|GetAllActorsOfClass "/Script/KFServerOverlaps.KF_Example04_Char"))
      (Utilities|IsValid (Utilities|Array|Get(acopy) _outactors)
        (:Is%20Valid
          (Variables|Default|SetSpawnTransform (Transformation|GetActorTransform (Utilities|Array|Get(acopy) _outactors))))
        (:Is%20Not%20Valid
          (bind _outactors_2 (Actor|GetAllActorsOfClass "/Script/Engine.PlayerStart"))
          (Variables|Default|SetSpawnTransform (Transformation|GetActorTransform (Utilities|Array|Get(acopy) _outactors_2)))))
      (bind _returnvalue (Game|SpawnActorfromClass "/Script/KFServerOverlaps.KF_Example04_Char" (Math|Transform|MakeTransform (+ (.location (Variables|Default|GetSpawnTransform)) (Math|Vector|MakeVector (select (Math|Random|RandomBool) (Math|Random|RandomFloatinRange 5e+01 1.5e+02) (Math|Random|RandomFloatinRange -5e+01 -1.5e+02)) (Math|Random|RandomFloatinRange -5e+01 -1.5e+02) 0.0)) (.rotation (Variables|Default|GetSpawnTransform)) (.scale (Variables|Default|GetSpawnTransform))) "AdjustIfPossibleButAlwaysSpawn" (Variables|Default|GetLocal_NewPlayer) 0))
      (Pawn|Possess (Variables|Default|GetLocal_NewPlayer) _returnvalue))))

(fn ConstructionScript)