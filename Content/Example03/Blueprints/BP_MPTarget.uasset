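; BP_MPTarget is a shootable target for a multiplayer example that triggers an animation on a linked ConnectedVictim actor.
; When a BP_MPProjectile hits its mesh, it plays a 2D snap sound and calls ServerIgniteAnimation on the victim.
; A timeline lerps the mesh through a half-turn rotation, playing at BeginPlay and driven forward or in reverse by PlayReverseAnim.
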(event OnComponentHit(StaticMesh)
  (params (HitComponent :type Primitive%20Component%20Object%20Reference) (OtherActor :type Actor%20Object%20Reference) (OtherComp :type Primitive%20Component%20Object%20Reference) (NormalImpulse :type Vector :default "0, 0, 0") (Hit :type Hit%20Result%20Structure%20%28by%20ref%29))
  (Utilities|Casting|CastToBP_MPProjectile OtherActor)
  (Audio|PlaySound2D "/Engine/VREditor/Sounds/UI/Object_Snaps_To_Grid.Object_Snaps_To_Grid" 1.0 1.0 0.0 0 0)
  (Default|ServerIgniteAnimation (Variables|Default|GetConnectedVictim)))

(event Custom|PlayReverseAnim
  (params (bForward? :type Boolean))
  (if bForward?
    (bind _0_1 (Timeline|Timeline_0 Play)
      (:Update
        (Transformation|SetRelativeRotation (Variables|Default|GetStaticMesh) (Math|Rotator|Lerp(Rotator) "0, 0, 0" "180.000000, 0, 0" _0_1 true) false false)))
    (else
      (Timeline|Timeline_0 Reverse))))

(event EventBeginPlay
  (bind _0_1 (Timeline|Timeline_0 PlayFromStart)
    (:Update
      (Transformation|SetRelativeRotation (Variables|Default|GetStaticMesh) (Math|Rotator|Lerp(Rotator) "0, 0, 0" "180.000000, 0, 0" _0_1 true) false false))))

(fn ConstructionScript)