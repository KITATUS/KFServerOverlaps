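; BP_Chair is a chair actor that plays a timed ignite particle effect across a networked game.
; A server ignite event passes through a DoOnce gate, calls multicast events to activate the particle system and deactivate it three seconds later, then resets after a short delay.
; The gate keeps repeat requests from restarting the effect while it runs.
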(event Custom|MC_Ignite
  (Components|Activation|Activate (Variables|Default|GetParticleSystem) true))

(event Custom|MC_StopIgnite
  (Components|Activation|Deactivate (Variables|Default|GetParticleSystem)))

(event Custom|Server_IgniteAnimation
  (Utilities|FlowControl|DoOnce false :!label _label
    (:Completed
      (CallFunction|MCIgnite)
      (Utilities|FlowControl|Delay 3.0)
      (CallFunction|MCStopIgnite)
      (Utilities|FlowControl|Delay 0.2)
      (goto _label Reset))))

(fn ConstructionScript)